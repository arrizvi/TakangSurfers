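; BP_ControllerNew is a controller Blueprint that saves and loads the player's score through a save slot.
; SaveGame loads or creates a MySaveGame object, copies CoinScore from player 0's BP_TakangCharacter into its Score, and writes the slot without comparing against the stored value.
; LoadGame reads that Score back into the character's HIghScore when the slot exists.
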(fn ConstructionScript)

(fn SaveGame
  (bind _returnvalue (SaveGame|DoesSaveGameExist (Variables|Default|GetSlot%20Name)))
  (if _returnvalue
    (bind _returnvalue_2 (SaveGame|LoadGamefromSlot (Variables|Default|GetSlot%20Name)))
    (Variables|Default|SetSaveRef _returnvalue_2)
    (else
      (bind _returnvalue_3 (SaveGame|CreateSaveGameObject "/Game/BPClass/MySaveGame.MySaveGame_C"))
      (Variables|Default|SetSaveRef _returnvalue_3)))
  (bind _asmy_save_game (Utilities|Casting|CastToMySaveGame (Variables|Default|GetSaveRef)))
  (bind _asbp_takang_character (Utilities|Casting|CastToBP_TakangCharacter (Game|Player|GetPlayerPawn 0)))
  (Variables|/Game/BPClass/MySaveGame.MySaveGame_C|SetScore _asmy_save_game (Variables|/Script/Takang.Takang_Hero|GetCoinScore _asbp_takang_character))
  (SaveGame|SaveGametoSlot (Variables|Default|GetSaveRef) (Variables|Default|GetSlot%20Name)))

(fn LoadGame
  (bind _returnvalue (SaveGame|DoesSaveGameExist (Variables|Default|GetSlot%20Name)))
  (if _returnvalue
    (bind _returnvalue_2 (SaveGame|LoadGamefromSlot (Variables|Default|GetSlot%20Name)))
    (bind _asmy_save_game (Utilities|Casting|CastToMySaveGame _returnvalue_2))
    (bind _asbp_takang_character (Utilities|Casting|CastToBP_TakangCharacter (Game|Player|GetPlayerPawn 0)))
    (Variables|/Game/BPClass/BP_TakangCharacter.BP_TakangCharacter_C|SetHIghScore _asbp_takang_character (Variables|/Game/BPClass/MySaveGame.MySaveGame_C|GetScore _asmy_save_game))))