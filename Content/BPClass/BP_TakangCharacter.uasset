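; Player character Blueprint for Takang that also sets up the game's menu and screen widgets.
; On BeginPlay it creates the UI widgets, shows the main menu with the game paused and cursor visible, and caches the custom player controller.
; Events show an animated game-over screen and chain two death montages by waiting out the first's length.
; The construction script assigns the Tak_Anim animation class to the mesh.
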(event Custom|GAmeOVer
  (bind _gameoverscreen (Variables|Default|GetGameOverScreen))
  (UserInterface|Viewport|AddtoViewport _gameoverscreen 0)
  (Default|PlayAnim _gameoverscreen))

(event EventPlayDeath
  (bind _returnvalue (Animation|PlayAnimMontage "/Game/Character/NewFolder/deathMontage.deathMontage" 1.0 "None"))
  (Utilities|FlowControl|Delay _returnvalue)
  (Animation|PlayAnimMontage "/Game/Character/NewFolder/CompleteDeath.CompleteDeath" 1.0 "None"))

(event EventBeginPlay
  ;[1 1 1] Comment
  (Utilities|FlowControl|Sequence
    (:then_0
      (bind _returnvalue (UserInterface|CreateWidget "/Game/UI/WBP/MainScreen.MainScreen_C"))
      (bind _output_get (Variables|Default|SetMainMenueWidget _returnvalue))
      (UserInterface|Viewport|AddtoViewport _output_get 0)
      (Game|SetGamePaused true)
      (bind _returnvalue_2 (UserInterface|CreateWidget "/Game/UI/WBP/GameScreen.GameScreen_C"))
      (Variables|Default|SetINGameWidget _returnvalue_2)
      (bind _returnvalue_3 (UserInterface|CreateWidget "/Game/UI/WBP/PauseGameMenue.PauseGameMenue_C"))
      (Variables|Default|SetPauseMenueWidget _returnvalue_3)
      (bind _returnvalue_4 (UserInterface|CreateWidget "/Game/UI/WBP/CharacterSelectionScreen.CharacterSelectionScreen_C"))
      (Variables|Default|SetCharacterSelectionScreen _returnvalue_4)
      (bind _returnvalue_5 (UserInterface|CreateWidget "/Game/UI/WBP/GAmeOver.GAmeOver_C"))
      (Variables|Default|SetGameOverScreen _returnvalue_5)
      (bind _returnvalue_6 (UserInterface|CreateWidget "/Game/UI/WBP/SettingsScreen.SettingsScreen_C"))
      (Variables|Default|SetsettingsScreenRef _returnvalue_6)
      (bind _asbp_controller_new (Utilities|Casting|CastToBP_ControllerNew (Game|GetPlayerController 0)))
      (Variables|Default|SetAs%20My%20Controller%20New _asbp_controller_new))
    (:then_1
      (Variables|/Script/Engine.PlayerController|SetbShowMouseCursor (Game|GetPlayerController 0) true))))

(fn ConstructionScript
  (Class|SkeletalMeshComponent|SetAnimClass (Variables|Character|GetMesh) "/Game/BPClass/Tak_Anim.Tak_Anim_C"))

(fn Alpha
  (params (NewParam :type Integer)))